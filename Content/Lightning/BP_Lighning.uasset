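; Lightning actor that replays a Niagara bolt effect and a spotlight flash at random intervals of several seconds.
; On BeginPlay it positions and rotates the effect, unpauses it and starts the Flashing timeline, whose track drives the spotlight's world Z height rather than its intensity.
; A random Delay on the timeline's Update output loops back to replay it; the node that would pause the effect is unconnected.
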(event `self.ReceiveBeginPlay`
  (bind _spotlightcomponent (`self.SpotLightComponent`))
  (bind _ns_lightning (`self.NS_Lightning`))
  (bind (_returnvalue_x _returnvalue_y) (`KismetMathLibrary.BreakVector` (`SceneComponent.K2_GetComponentLocation` _spotlightcomponent)))
  (`SceneComponent.K2_SetWorldLocation` _ns_lightning (`self.New Location`) false false)
  (`SceneComponent.K2_SetWorldRotation` _ns_lightning (`self.New Rotation`) false false)
  (`NiagaraComponent.SetPaused` (`self.NS_Lightning`) false :!label _label)
  (bind (_direction _newtrack_0) (`Timeline|Flashing` :!via `PlayFromStart`)
    (:`Update`
      (`SceneComponent.K2_SetWorldLocation` _spotlightcomponent (`KismetMathLibrary.MakeVector` _returnvalue_x _returnvalue_y _newtrack_0) false false)
      (`KismetSystemLibrary.Delay` (`KismetMathLibrary.RandomFloatInRange` 5.0 10.0))
      (goto _label))))

(fn `UserConstructionScript`)