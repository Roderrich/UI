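; Camera-point actor for the LAN menu that blends the player's view between referenced cameras, apparently for character select.
; An index event validates the entry in CameraReference, passes it to MoveCamera and prints the index.
; MoveCamera disables its own collision, enables the target's and runs a timed view-target blend on player controller 0.
; BeginPlay only casts its widget component's content to WBP_CHSelectLAN.
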(event `self.ReceiveBeginPlay`
  (cast `/Game/LAN/WBP_CHSelectLAN` (`WidgetComponent.GetUserWidgetObject` (`self.Widget`))))

(event `CustomEvent_0`
  (params (CameraInteger :type Integer))
  (if (`KismetArrayLibrary.Array_IsValidIndex` (`self.CameraReference`) CameraInteger)
    (`self.MoveCamera` (`|GetArrayItem` (`self.CameraReference`) CameraInteger))
    (`KismetSystemLibrary.PrintString` (`KismetStringLibrary.Conv_IntToString` CameraInteger))))

(event `MoveCamera`
  (params (NewParam :type "/Game/LAN/BPC_Camera Object Reference"))
  (`self.SetActorEnableCollision` false)
  (`self.SetActorEnableCollision` NewParam true)
  (`PlayerController.SetViewTargetWithBlend` (`GameplayStatics.GetPlayerController` 0) NewParam 3.0 "VTBlend_PreBlended" 2.0 false))

(fn `UserConstructionScript`)