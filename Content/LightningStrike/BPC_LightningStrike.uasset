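; BPC_LightningStrike is an actor that repeatedly spawns lightning strikes at random points in a flat box around itself.
; Each cycle spawns a Niagara effect, destroys it after a random delay, then loops.
; In parallel, a delayed branch briefly teleports the Sphere component to the strike point, then back to a fixed parking location.
; The Sphere's overlap event is empty, so strikes apply no effect here.
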(event `self.ReceiveBeginPlay`
  (`SceneComponent.K2_SetWorldLocation` (`self.Sphere`) (-400.0 0.0 0.0) false true)
  (bind _output_get (set `self.NewLocation` (`KismetMathLibrary.RandomPointInBoundingBox` (`self.K2_GetActorLocation`) (1800.0 1500.0 0.1)) :!label _label))
  (`|ExecutionSequence`
    (:`then_0`
      (bind _returnvalue (`NiagaraFunctionLibrary.SpawnSystemAtLocation` "/Game/asd/NS_IDKIMGOINGINSAINE.NS_IDKIMGOINGINSAINE" _output_get))
      (`KismetSystemLibrary.Delay` (`KismetMathLibrary.RandomFloatInRange` 3.6 8.0))
      (`ActorComponent.K2_DestroyComponent` _returnvalue)
      (goto _label))
    (:`then_1`
      (`KismetSystemLibrary.Delay` 3.3)
      (`SceneComponent.K2_SetWorldLocation` (`self.Sphere`) (`self.NewLocation`) false true)
      (`KismetSystemLibrary.Delay` 0.3)
      (`SceneComponent.K2_SetWorldLocation` (`self.Sphere`) (-400.0 0.0 0.0) false true))))

(event `self.Sphere.OnComponentBeginOverlap`
  (params (OverlappedComponent :type "PrimitiveComponent Object Reference") (OtherActor :type "Actor Object Reference") (OtherComp :type "PrimitiveComponent Object Reference") (OtherBodyIndex :type Integer) (bFromSweep :type Boolean) (SweepResult :type "HitResult Structure (by ref)")))

(fn `UserConstructionScript`)