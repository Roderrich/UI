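; Game manager Blueprint that sets up local multiplayer when play begins, creating players based on the PlayerStart actors in the level.
; For each PlayerStart it creates a local player, stores it by index, adds an Enhanced Input mapping context and calls Possess on that player's controller.
; NumberOfPlayers holds the last PlayerStart index rather than the count.
; A SpawnActor node is left unconnected, so no pawns are spawned here.
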(event `self.ReceiveBeginPlay`
  (bind _outactors (`GameplayStatics.GetAllActorsOfClass` "/Script/Engine.PlayerStart"))
  (set `self.NumberOfPlayers` (`KismetArrayLibrary.Array_LastIndex` _outactors))
  (for (_ _array_index) _outactors
    (bind _output_get (set `self.PlayerIndex` _array_index))
    (bind _returnvalue (`GameplayStatics.CreatePlayer` _output_get))
    (`KismetArrayLibrary.Array_Set` (`self.LocalPlayer`) _output_get _returnvalue)
    (bind _returnvalue_2 (pcsubsystem `EnhancedInputLocalPlayerSubsystem` (`GameplayStatics.GetPlayerController` _output_get)))
    (`/Engine/EditorBlueprintResources/StandardMacros.IsValid` _returnvalue_2
      (:`Is Valid`
        (`EnhancedInputSubsystemInterface.AddMappingContext` _returnvalue_2 null 0 (struct))
        (`Controller.Possess` (`GameplayStatics.GetPlayerController` (`self.PlayerIndex`)) null)))))

(fn `UserConstructionScript`)