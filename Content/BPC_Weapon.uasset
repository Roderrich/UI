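; Weapon component Blueprint that counts attacks into a three-hit combo.
; Each Attack draws a debug visibility trace, its result unused, and increments the count, which a 0.75-second retriggerable delay resets after inactivity.
; The third attack launches player character 0, not a traced target, along the given direction scaled by Knockback, then resets the count.
; Montage selection and a pawn object trace noted for LAN are unconnected.
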(event `Attack`
  (params (Start :type "Vector Structure") (End :type "Vector Structure") (Direction :type "Vector Structure"))
  ;[1 1 1] Combo Counter
  ;;[1 1 1] For Presentation visually
  (`KismetSystemLibrary.LineTraceSingle` :`Start` Start :`End` End :`TraceChannel` "TraceTypeQuery1" :`DrawDebugType` "ForDuration")
  (`/Engine/EditorBlueprintResources/StandardMacros.IncrementInt` (`self.ComboCount`)
    (:`  `
      (if (== (`self.ComboCount`) 3)
        (`Character.LaunchCharacter` (`GameplayStatics.GetPlayerCharacter` 0) (* Direction (`self.Knockback`)) true false)
        (set `self.ComboCount` 0)
        (else
          (`KismetSystemLibrary.RetriggerableDelay` 0.75)
          (set `self.ComboCount` 0))))))